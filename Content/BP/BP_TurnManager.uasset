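; BP_TurnManager starts a battle shortly after play begins and keeps the turn icon on the player's HUD updated.
; After staged delays, it calls StartBattle, then caches the MainHud from the player's BP_CombatCharacter pawn.
; A looping half-second timer repeatedly pushes IconTurn to the HUD's TurnIcon, so the display refreshes by polling.
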(event `self.ReceiveBeginPlay`
  (`KismetSystemLibrary.Delay` 2.0)
  (`self.StartBattle`)
  (`KismetSystemLibrary.Delay` 1.0)
  (bind _asbp_combat_character (cast `/Game/BP/BP_CombatCharacter` (`GameplayStatics.GetPlayerPawn` 0)))
  (set `self.Main Hud` (`/Game/BP/BP_CombatCharacter.MainHud` _asbp_combat_character))
  (bind _output_get (set `self.Icon Turn` (`self.IconTurn`)))
  (`/Game/BP/HUD_Main.TurnIcon` (`self.Main Hud`) _output_get)
  (`KismetSystemLibrary.K2_SetTimerDelegate` (delegate `adasd`) 0.5 true))

(event `adasd`
  (bind _output_get (set `self.Icon Turn` (`self.IconTurn`)))
  (`/Game/BP/HUD_Main.TurnIcon` (`self.Main Hud`) _output_get))

(fn `UserConstructionScript`)