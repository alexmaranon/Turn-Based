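; Player combat character Blueprint that loads abilities from the player state into its ability widget and shows a marker on the targeted enemy.
; On BeginPlay, after a short delay, it spawns BP_Target at an enemy and starts a looping timer.
; The timer updates HUD HP, fires a camera shake and moves the marker, falling back to the first Enemies entry.
; Target cycling and energy-cost ability montage logic exist but are disconnected.
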(event `self.ReceiveBeginPlay`
  (`KismetArrayLibrary.Array_Clear` (`self.DT_Abilities`))
  (`KismetSystemLibrary.Delay` 0.2)
  (bind _asps (cast `/Game/BP/PS` (`GameplayStatics.GetPlayerState` 0)))
  (bind _output_get (set `self.As PS` _asps))
  (bind _returnvalue (`PlayerStates.GetCurrentAbilities` _output_get))
  (for _array_element _returnvalue
    (`KismetArrayLibrary.Array_Add` (`self.DT_Abilities`) (`AttackAbility.AttackAttributes` _array_element)))
  (bind _asw_character_abilities (cast `/Game/BP/W_CharacterAbilities` (`WidgetComponent.GetWidget` (`self.Abilities`))))
  (bind _output_get_2 (set `self.As W Character Abilities` _asw_character_abilities))
  (`/Game/BP/W_CharacterAbilities.Init` _output_get_2 (`self.DT_Abilities`))
  (bind _outactors (`GameplayStatics.GetAllActorsOfClass` "/Game/BP/BP_Enemies.BP_Enemies_C"))
  (set `self.Target` _outactors)
  (bind _output (`|GetArrayItem` _outactors (`self.TargetVal`)))
  (bind _returnvalue_2 (`|SpawnActorFromClass` "/Game/BP/BP_Target.BP_Target_C" (`KismetMathLibrary.MakeTransform` (- (`self.K2_GetActorLocation` _output) (/ (`KismetMathLibrary.MakeVector` 0.0 0.0 (.z (`.BoxExtent` (`self.GetActorBounds` _output false false)))) 2.0))) "AlwaysSpawn" "MultiplyWithRoot" null null))
  (set `self.TagetBP` _returnvalue_2)
  (bind _ashud_main (cast `/Game/BP/HUD_Main` (`PlayerController.GetHUD` (`GameplayStatics.GetPlayerController` 0))))
  (set `self.MainHud` _ashud_main)
  (`KismetSystemLibrary.K2_SetTimerDelegate` (delegate `Update`) 0.1 true))

(event `Update`
  (bind _enemies (`self.Enemies`))
  (bind _targetenemy (`self.TargetEnemy`))
  (`/Game/BP/HUD_Main.UpdateHP` (`self.MainHud`) (`CharacterCombatComponent.CurrentHP` (`self.CharacterCombat`)) (`CharacterCombatComponent.MaxHP` (`self.CharacterCombat`)))
  (`PlayerController.ClientStartCameraShake` :`self` (`GameplayStatics.GetPlayerController` 0) :`Shake` "/Game/BP/CameraShake.CameraShake_C")
  (if (and (`KismetSystemLibrary.IsValid` _targetenemy) (`KismetSystemLibrary.IsValid` (`self.TagetBP`)))
    (`self.K2_SetActorLocation` (`self.TagetBP`) (- (`self.K2_GetActorLocation` _targetenemy) (/ (`KismetMathLibrary.MakeVector` 0.0 0.0 (.z (`.BoxExtent` (`self.GetActorBounds` _targetenemy false false)))) 2.0)) false false)
    (elif (> (`KismetArrayLibrary.Array_Length` _enemies) 0)
      (set `self.TargetEnemy` (`|GetArrayItem` _enemies)))))

(event `EnhancedInput|/Game/ThirdPerson/Input/Actions/IA_ChangeTarget`
  (params (ActionValue :type "Float (double-precision)") (ElapsedSeconds :type "Float (double-precision)") (TriggeredSeconds :type "Float (double-precision)") (InputAction :type "InputAction Object Reference" :default "/Game/ThirdPerson/Input/Actions/IA_ChangeTarget.IA_ChangeTarget")))

(fn `UserConstructionScript`)