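; Enemy Blueprint that fills its Abilities widget with attack data taken from a player state at spawn.
; On BeginPlay it clears DTAbilities, waits briefly, then reads the current abilities from the PS player state at index 0, not from the enemy itself.
; It collects each ability's AttackAttributes into DTAbilities and passes that array to W_CharacterAbilities for initialization.
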(event `self.ReceiveBeginPlay`
  (`KismetArrayLibrary.Array_Clear` (`self.DT_Abilities`))
  (`KismetSystemLibrary.Delay` 0.2)
  (bind _asps (cast `/Game/BP/PS` (`GameplayStatics.GetPlayerState` 0)))
  (bind _output_get (set `self.As PS` _asps))
  (bind _returnvalue (`PlayerStates.GetCurrentAbilities` _output_get))
  (for _array_element _returnvalue
    (`KismetArrayLibrary.Array_Add` (`self.DT_Abilities`) (`AttackAbility.AttackAttributes` _array_element)))
  (bind _asw_character_abilities (cast `/Game/BP/W_CharacterAbilities` (`WidgetComponent.GetWidget` (`self.Abilities`))))
  (bind _output_get_2 (set `self.As W Character Abilities` _asw_character_abilities))
  (`/Game/BP/W_CharacterAbilities.Init` _output_get_2 (`self.DT_Abilities`)))

(fn `UserConstructionScript`)